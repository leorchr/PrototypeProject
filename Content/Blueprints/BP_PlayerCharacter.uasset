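; Player character Blueprint that handles Enhanced Input for movement, camera look, sprint, crouch and a spell effect.
; Movement follows control-rotation yaw only, keeping it on the horizontal plane, while look feeds controller pitch and yaw.
; Sprint swaps max walk speed while held, and crouch toggles on each press.
; Casting spawns a spell particle system at the mesh location, then deactivates it after a short delay.
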(event `EnhancedInput|/Game/Inputs/InputActions/IA_Move`
  (params (ActionValue :type "Vector2D Structure") (ElapsedSeconds :type "Float (double-precision)") (TriggeredSeconds :type "Float (double-precision)") (InputAction :type "InputAction Object Reference" :default "/Game/Inputs/InputActions/IA_Move.IA_Move"))
  (bind _returnvalue (`KismetMathLibrary.MakeRotator` 0.0 0.0 (.yaw (`self.GetControlRotation`))))
  (:`Triggered`
    (`self.AddMovementInput` (`KismetMathLibrary.GetForwardVector` _returnvalue) ActionValue_X)
    (`self.AddMovementInput` (`KismetMathLibrary.GetRightVector` _returnvalue) ActionValue_Y)))

(event `EnhancedInput|/Game/Inputs/InputActions/IA_Look`
  (params (ActionValue :type "Vector2D Structure") (ElapsedSeconds :type "Float (double-precision)") (TriggeredSeconds :type "Float (double-precision)") (InputAction :type "InputAction Object Reference" :default "/Game/Inputs/InputActions/IA_Look.IA_Look"))
  (:`Triggered`
    (`self.AddControllerPitchInput` ActionValue_Y)
    (`self.AddControllerYawInput` ActionValue_X)))

(event `EnhancedInput|/Game/Inputs/InputActions/IA_Sprint`
  (params (ActionValue :type Boolean) (ElapsedSeconds :type "Float (double-precision)") (TriggeredSeconds :type "Float (double-precision)") (InputAction :type "InputAction Object Reference" :default "/Game/Inputs/InputActions/IA_Sprint.IA_Sprint"))
  (:`Triggered`
    (set `CharacterMovementComponent.MaxWalkSpeed` (`self.SprintSpeed`) (`self.CharacterMovement`)))
  (:`Canceled`
    (set `CharacterMovementComponent.MaxWalkSpeed` (`self.WalkSpeed`) (`self.CharacterMovement`) :!label _label))
  (:`Completed`
    (goto _label)))

(event `EnhancedInput|/Game/Inputs/InputActions/IA_Crouch`
  (params (ActionValue :type Boolean) (ElapsedSeconds :type "Float (double-precision)") (TriggeredSeconds :type "Float (double-precision)") (InputAction :type "InputAction Object Reference" :default "/Game/Inputs/InputActions/IA_Crouch.IA_Crouch"))
  (:`Started`
    (if (`self.IsCrouched`)
      (`self.UnCrouch`)
      (set `self.IsCrouched` false)
      (else
        (`self.Crouch`)
        (set `self.IsCrouched` true)))))

(event `EnhancedInput|/Game/Inputs/InputActions/IA_Spell`
  (params (ActionValue :type Boolean) (ElapsedSeconds :type "Float (double-precision)") (TriggeredSeconds :type "Float (double-precision)") (InputAction :type "InputAction Object Reference" :default "/Game/Inputs/InputActions/IA_Spell.IA_Spell"))
  (:`Started`
    (bind _returnvalue (`NiagaraFunctionLibrary.SpawnSystemAtLocation` "/Game/FX/FXS_Spell.FXS_Spell" (`SceneComponent.K2_GetComponentLocation` (`self.Mesh`))))
    (set `self.System` _returnvalue)
    (`KismetSystemLibrary.Delay` 0.5)
    (`ActorComponent.Deactivate` (`self.System`))))

(fn `UserConstructionScript`)