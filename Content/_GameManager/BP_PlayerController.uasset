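; Player controller that handles Enhanced Input for BP_PlayerCharacter: movement, look, sprint, crouch and spell casting.
; BeginPlay adds the main mapping context and caches the controlled character and its movement component.
; Movement follows control yaw only, sprint swaps MaxWalkSpeed between the character's walk and sprint speeds, and crouch toggles.
; Spell input calls CastProjectile on press and FireProjectile on release, with debug prints.
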(event `self.ReceiveBeginPlay`
  (`EnhancedInputSubsystemInterface.AddMappingContext` (subsystem `EnhancedInputLocalPlayerSubsystem`) "/Game/Inputs/IMC_Main.IMC_Main" 0 (struct))
  (bind _asbp_player_character (cast `/Game/_GameManager/BP_PlayerCharacter` (`self.K2_GetPawn`)))
  (set `self.PlayerCharacter` _asbp_player_character)
  (set `self.Character Movement` (`Character.CharacterMovement` _asbp_player_character)))

(event `EnhancedInput|/Game/Inputs/InputActions/IA_Move`
  (params (ActionValue :type "Vector2D Structure") (ElapsedSeconds :type "Float (double-precision)") (TriggeredSeconds :type "Float (double-precision)") (InputAction :type "InputAction Object Reference" :default "/Game/Inputs/InputActions/IA_Move.IA_Move"))
  (bind _returnvalue (`KismetMathLibrary.MakeRotator` 0.0 0.0 (.yaw (`self.GetControlRotation`))))
  (:`Triggered`
    (`Pawn.AddMovementInput` (`self.K2_GetPawn`) (`KismetMathLibrary.GetForwardVector` _returnvalue) ActionValue_X false)
    (`Pawn.AddMovementInput` (`self.K2_GetPawn`) (`KismetMathLibrary.GetRightVector` _returnvalue) ActionValue_Y false)))

(event `EnhancedInput|/Game/Inputs/InputActions/IA_Look`
  (params (ActionValue :type "Vector2D Structure") (ElapsedSeconds :type "Float (double-precision)") (TriggeredSeconds :type "Float (double-precision)") (InputAction :type "InputAction Object Reference" :default "/Game/Inputs/InputActions/IA_Look.IA_Look"))
  (bind _returnvalue (`self.K2_GetPawn`))
  (:`Triggered`
    (`Pawn.AddControllerPitchInput` _returnvalue ActionValue_Y)
    (`Pawn.AddControllerYawInput` _returnvalue ActionValue_X)))

(event `EnhancedInput|/Game/Inputs/InputActions/IA_Sprint`
  (params (ActionValue :type Boolean) (ElapsedSeconds :type "Float (double-precision)") (TriggeredSeconds :type "Float (double-precision)") (InputAction :type "InputAction Object Reference" :default "/Game/Inputs/InputActions/IA_Sprint.IA_Sprint"))
  (:`Triggered`
    (set `CharacterMovementComponent.MaxWalkSpeed` (`/Game/_GameManager/BP_PlayerCharacter.SprintSpeed` (`self.PlayerCharacter`)) (`self.Character Movement`)))
  (:`Canceled`
    (set `CharacterMovementComponent.MaxWalkSpeed` (`/Game/_GameManager/BP_PlayerCharacter.WalkSpeed` (`self.PlayerCharacter`)) (`self.Character Movement`) :!label _label))
  (:`Completed`
    (goto _label)))

(event `EnhancedInput|/Game/Inputs/InputActions/IA_Crouch`
  (params (ActionValue :type Boolean) (ElapsedSeconds :type "Float (double-precision)") (TriggeredSeconds :type "Float (double-precision)") (InputAction :type "InputAction Object Reference" :default "/Game/Inputs/InputActions/IA_Crouch.IA_Crouch"))
  (bind _playercharacter (`self.PlayerCharacter`))
  (:`Started`
    (if (`Character.bIsCrouched` _playercharacter)
      (`Character.UnCrouch` _playercharacter)
      (else
        (`Character.Crouch` _playercharacter)))))

(event `EnhancedInput|/Game/Inputs/InputActions/IA_Spell`
  (params (ActionValue :type Boolean) (ElapsedSeconds :type "Float (double-precision)") (TriggeredSeconds :type "Float (double-precision)") (InputAction :type "InputAction Object Reference" :default "/Game/Inputs/InputActions/IA_Spell.IA_Spell"))
  (:`Started`
    (`KismetSystemLibrary.PrintString` "Cast")
    (bind _asbp_player_character (cast `/Game/_GameManager/BP_PlayerCharacter` (`self.K2_GetPawn`)))
    (`/Game/_GameManager/BP_PlayerCharacter.CastProjectile` _asbp_player_character))
  (:`Completed`
    (`KismetSystemLibrary.PrintString` "Fire")
    (bind _asbp_player_character_2 (cast `/Game/_GameManager/BP_PlayerCharacter` (`self.K2_GetPawn`)))
    (`/Game/_GameManager/BP_PlayerCharacter.FireProjectile` _asbp_player_character_2)))

(fn `UserConstructionScript`)